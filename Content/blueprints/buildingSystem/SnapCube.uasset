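; SnapCube is a building-system actor that snaps itself to a grid whenever its construction script runs.
; The script rounds each axis of location, rotation and scale to fixed increments using GridSnapFloat.
; It reads world-space values but writes them with SetActorRelativeTransform, so the two match only when the actor has no transformed parent.
; The event graph holds only disabled placeholder events, so the Blueprint adds no gameplay logic.
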(event EventBeginPlay)

(event Collision|EventActorBeginOverlap
  (params (OtherActor :type Actor%20Object%20Reference)))

(event EventTick
  (params (DeltaSeconds :type Float%20%28single-precision%29)))

(fn ConstructionScript
  (bind _returnvalue (Transformation|GetActorLocation))
  (bind _returnvalue_2 (Transformation|GetActorScale3D))
  (bind _returnvalue_3 (Transformation|GetActorRotation))
  (bind (_roll _pitch _yaw) (Math|Rotator|BreakRotator _returnvalue_3))
  (bind (_x _y _z) (Math|Vector|BreakVector _returnvalue))
  (bind (_x_2 _y_2 _z_2) (Math|Vector|BreakVector _returnvalue_2))
  (Transformation|SetActorRelativeTransform (Math|Transform|MakeTransform (Math|Vector|MakeVector (Math|Float|SnapToGrid(Float) _x 5e+01) (Math|Float|SnapToGrid(Float) _y 5e+01) (Math|Float|SnapToGrid(Float) _z 5e+01)) (Math|Rotator|MakeRotator (Math|Float|SnapToGrid(Float) _roll 45.0) (Math|Float|SnapToGrid(Float) _pitch 45.0) (Math|Float|SnapToGrid(Float) _yaw 45.0)) (Math|Vector|MakeVector (Math|Float|SnapToGrid(Float) _x_2 0.5) (Math|Float|SnapToGrid(Float) _y_2 0.5) (Math|Float|SnapToGrid(Float) _z_2 0.5))) false false))